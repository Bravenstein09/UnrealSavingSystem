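; BP_Objective represents a single objective in the quest system, holding its name, data, active state and completion state.
; ActivateObjective marks the objective active only if it is not already complete, then fires OnActivated with itself, even for a completed objective.
; Getter functions expose the name, both state flags and the objective data; this file contains no logic that sets completion.
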(event Custom|ActivateObjective
  (bind _self self)
  (Variables|Default|SetIsActive (not (Variables|Default|GetIsComplete)))
  (Default|CallOnActivated _self _self))

(fn GetObjectiveName
  (return (Variables|Default|GetObjectiveName)))

(fn GetIsComplete
  (return (Variables|Default|GetIsComplete)))

(fn GetIsActive
  (return (Variables|Default|GetIsActive)))

(fn GetData
  (return (Variables|Default|GetObjectiveData)))