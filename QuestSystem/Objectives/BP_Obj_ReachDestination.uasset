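; Quest objective Blueprint that completes when the Destination actor registers an overlap.
; On activation it runs the parent logic, then, if not yet complete and Destination is valid, binds to that actor's begin-overlap event.
; The overlap handler does not filter the overlapping actor, so any overlap sets IsComplete and broadcasts OnCompleted with itself.
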(event Custom|CustomEvent_0
  (params (OverlappedActor :type Actor%20Object%20Reference) (OtherActor :type Actor%20Object%20Reference))
  (bind _self self)
  (if true
    (Variables|Default|SetIsComplete true)
    (Default|CallOnCompleted _self _self)))

(event EventActivateObjective
  (|CallParentFunction)
  (if (not (CallFunction|GetIsComplete))
    (bind _destination (Variables|Default|GetDestination)
      (:then
        (Collision|BindEventtoOnActorBeginOverlap _destination (delegate Custom|CustomEvent_0)))
      (:else))))

(fn GetIsComplete
  (return (Variables|Default|GetIsComplete)))