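; Test quest for the quest system that builds a root objective collection with one reach-destination objective per entry in Destinations.
; Overrides of the construction, population and save-name functions restore each objective's name, completion and data from saved data, keyed by "TestingQuest" or destination display name.
; Tick prints debug text for root completion, active objectives and whether saved data exists.
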(event EventBeginPlay
  (|CallParentFunction) ; This node is disabled and will not be called.\nDrag off pins to build functionality.
)

(event Collision|EventActorBeginOverlap
  (params (OtherActor :type Actor%20Object%20Reference)))

(event EventTick
  (params (DeltaSeconds :type Float%20%28single-precision%29))
  (bind _rootobjectivecollection (CallFunction|GetRootObjectiveCollection))
  (Utilities|FlowControl|Sequence
    (:then_0
      (Utilities|IsValid _rootobjectivecollection
        (:Is%20Valid
          (Development|PrintText (Utilities|Text|FormatText "{i} is complete {ii}" (Default|GetObjectiveName _rootobjectivecollection) (Utilities|String|SelectString "yes" "no" (Default|GetIsComplete _rootobjectivecollection))) true true "(R=0.000000,G=0.660000,B=1.000000,A=1.000000)" 0.0)
          (for _array_element (Variables|/Game/El/Blueprints/QuestSystem/Objectives/BP_ObjectiveCollection.BP_ObjectiveCollection_C|GetObjectives (CallFunction|GetRootObjectiveCollection))
            (Development|PrintText (Utilities|Text|FormatText "{i} is complete {ii}" (Default|GetObjectiveName _array_element) (Utilities|String|SelectString "yes" "no" (Default|GetIsComplete _array_element))) (Default|GetIsActive _array_element) (Default|GetIsActive _array_element) "(R=0.000000,G=0.660000,B=1.000000,A=1.000000)" 0.0)))))
    (:then_1
      (Development|PrintString (Utilities|String|SelectString "We have saved objective data" "We don't have saved objective data" (Utilities|Map|IsNotEmpty (Variables|Default|GetSavedObjectiveData))) true true "(R=0.000000,G=0.660000,B=1.000000,A=1.000000)" 0.0))))

(fn ConstructionScript
  (|CallParentFunction))

(fn PopulateObjectives
  (params (RootObjectiveCollection :type BP%20Objective%20Collection%20Object%20Reference))
  (for _array_element (Variables|Default|GetDestinations)
    (bind _returnvalue (Game|ConstructObjectfromClass "/Game/El/Blueprints/QuestSystem/Objectives/BP_Obj_ReachDestination.BP_Obj_ReachDestination_C" _array_element (.OutObjectiveName (Utilities|GetSavedObjectiveData (Utilities|GetDisplayName _array_element))) (.ObjectiveCompletion (Utilities|GetSavedObjectiveData (Utilities|GetDisplayName _array_element))) (.Data (Utilities|GetSavedObjectiveData (Utilities|GetDisplayName _array_element)))))
    (CallFunction|AddObjectivetoRootObjectiveCollection _returnvalue)
    (Development|PrintText (Utilities|Text|FormatText "Objective with name {i} was spawned with completion status {ii}" 0 (Utilities|String|SelectString "complete" "Incomplete" false)) true true "(R=1.000000,G=0.514554,B=0.454740,A=1.000000)" 1e+01)))

(fn ConstructRootObjectiveCollection
  (bind _returnvalue (Utilities|String|MakeLiteralString "TestingQuest"))
  (bind (_outobjectivename _objectivecompletion _data) (Utilities|GetSavedObjectiveData _returnvalue))
  (bind _returnvalue_2 (Game|ConstructObjectfromClass "/Game/El/Blueprints/QuestSystem/Objectives/BP_ObjectiveCollection.BP_ObjectiveCollection_C" false _outobjectivename _objectivecompletion _data))
  (return _returnvalue_2))

(fn GetUniqueSaveName
  (return (Utilities|String|MakeLiteralString "TestingQuest")))