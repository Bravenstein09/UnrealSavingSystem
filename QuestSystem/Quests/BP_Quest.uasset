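; Base quest Blueprint that owns a root objective collection and records objective progress for saving.
; After a short BeginPlay delay it builds, populates and activates the root, then binds completed and activated handlers, both empty here.
; Child classes must override construction and population, which only print errors here.
; Before saving, it recursively walks nested collections, storing completion and data by objective name, with the quest name as save key.
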(event Custom|RootObjectiveActivated
  (params (Objective :type BP%20Objective%20Object%20Reference)))

(event Custom|RootObjectiveCompleted
  (params (Objective :type BP%20Objective%20Object%20Reference)))

(event EventBeginPlay
  (Utilities|FlowControl|Delay 0.2)
  (bind _rootobjectivecollection (Private|ConstructRootObjectiveCollection))
  (bind _output_get (Variables|Private|SetRootObjectiveCollection _rootobjectivecollection))
  (Private|PopulateObjectives _output_get)
  (Default|ActivateObjective (Variables|Private|GetRootObjectiveCollection))
  (EventDispatchers|BindEventtoOnCompleted (Variables|Private|GetRootObjectiveCollection) (delegate Custom|RootObjectiveCompleted))
  (EventDispatchers|BindEventtoOnActivated (Variables|Private|GetRootObjectiveCollection) (delegate Custom|RootObjectiveActivated)))

(event EventOnBeforeSave
  (bind _rootobjectivecollection (Variables|Private|GetRootObjectiveCollection)
    (:then
      (Utilities|FlowControl|Sequence
        (:then_0
          (CallFunction|SaveObjectives _rootobjectivecollection))
        (:then_1
          (for _array_element (Variables|/Game/El/Blueprints/QuestSystem/Objectives/BP_ObjectiveCollection.BP_ObjectiveCollection_C|GetObjectives _rootobjectivecollection)
            (CallFunction|SaveObjectives _array_element)))))
    (:else)))

(fn ConstructionScript)

(fn ConstructRootObjectiveCollection
  (Development|PrintString "Error: CreateRootObjectiveCollectionCalledForBaseClass!!" true true "(R=1.000000,G=0.000000,B=0.000000,A=1.000000)")
  (return 0))

(fn PopulateObjectives
  (params (RootObjectiveCollection :type BP%20Objective%20Collection%20Object%20Reference))
  (Development|PrintString "Error:PopulateObjectivesCalledForBaseClass!!" true true "(R=1.000000,G=0.000000,B=0.000000,A=1.000000)")
  (return))

(fn GetRootObjectiveCollection
  (return (Variables|Private|GetRootObjectiveCollection)))

(fn AddObjectivetoRootObjectiveCollection
  (params (Objective :type BP%20Objective%20Object%20Reference))
  (Default|AddObjective (Variables|Private|GetRootObjectiveCollection) Objective))

(fn GetQuestName
  (return (Default|GetObjectiveName (Variables|Private|GetRootObjectiveCollection))))

(fn SaveObjectives
  (params (Objective :type BP%20Objective%20Object%20Reference))
  (bind _asbp_objective_collection (Utilities|Casting|CastToBP_ObjectiveCollection Objective)
    (:then
      (Utilities|FlowControl|Sequence
        (:then_0
          (CallFunction|SaveSingleObjective Objective))
        (:then_1
          (for _array_element (Variables|/Game/El/Blueprints/QuestSystem/Objectives/BP_ObjectiveCollection.BP_ObjectiveCollection_C|GetObjectives _asbp_objective_collection)
            (CallFunction|SaveObjectives _array_element)))))
    (:CastFailed
      (CallFunction|SaveSingleObjective Objective))))

(fn SaveSingleObjective
  (params (Objective :type BP%20Objective%20Object%20Reference))
  (Development|PrintString (Utilities|String|ToString(Text) (Utilities|Text|FormatText "Saved: {i} Status: {b}" (Default|GetObjectiveName Objective) (Utilities|String|SelectString "complete" "incomplete" (Default|GetIsComplete Objective)))))
  (Utilities|Map|Add (Variables|Default|GetSavedObjectiveCompletion) (Default|GetObjectiveName Objective) (Default|GetIsComplete Objective))
  (Utilities|Map|Add (Variables|Default|GetSavedObjectiveData) (Default|GetObjectiveName Objective) (Default|GetData Objective)))

(fn GetUniqueSaveName
  (return (Public|GetQuestName)))